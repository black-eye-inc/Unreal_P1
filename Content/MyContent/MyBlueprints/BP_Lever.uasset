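; BP_Lever is a one-way lever that the player switches on by interacting while inside its hitbox.
; Hitbox overlaps with BP_ThirdPersonCharacter set TouchingPlayer and toggle two E-icons, which spin and bob on a sine wave in Tick.
; Tick also polls and consumes the controller's PlayerInteract flag to set LeverOn and LeverPressed, and reapplies the up or down switch material every frame.
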(event OnComponentBeginOverlap(hitbox)
  (params (OverlappedComponent :type Primitive%20Component%20Object%20Reference) (OtherActor :type Actor%20Object%20Reference) (OtherComp :type Primitive%20Component%20Object%20Reference) (OtherBodyIndex :type Integer) (bFromSweep :type Boolean) (SweepResult :type Hit%20Result%20Structure%20%28by%20ref%29))
  ;[0.15 0.15 0.15 0.5] When the player enters touching range: set [touching_player] to TRUE...
  (Utilities|Casting|CastToBP_ThirdPersonCharacter OtherActor)
  (Variables|Default|Settouching_player true)
  ;[0.15 0.15 0.15 0.5] Toggle the visibility of the "E icon" so that it now is/isn't visible.
  (Rendering|ToggleVisibility (Variables|Default|GetIconE_p1) false))

(event OnComponentEndOverlap(hitbox)
  (params (OverlappedComponent :type Primitive%20Component%20Object%20Reference) (OtherActor :type Actor%20Object%20Reference) (OtherComp :type Primitive%20Component%20Object%20Reference) (OtherBodyIndex :type Integer))
  ;[0.15 0.15 0.15 0.5] When the player leaves touching range: set [touching_player] to FALSE...
  (Utilities|Casting|CastToBP_ThirdPersonCharacter OtherActor)
  (Variables|Default|Settouching_player false)
  ;[0.15 0.15 0.15 0.5] Toggle the visibility of the "E icon" so that it now is/isn't visible.
  (Rendering|ToggleVisibility (Variables|Default|GetIconE_p1) false))

(event EventTick
  (params (DeltaSeconds :type Float%20%28single-precision%29))
  (bind _switch (Variables|Default|GetSwitch))
  (bind _e_icon_center (Variables|Default|Gete_icon_center))
  (bind (_x _y _z) (Math|Vector|BreakVector _e_icon_center))
  ;[0.15 0.15 0.15 0.5] Every frame: make the "E-icon" rotate at a constant speed...
  (Transformation|AddLocalRotation (Variables|Default|GetIconE_p1) (Math|Rotator|MakeRotator 0.0 (* DeltaSeconds 4e+01) 0.0) false false)
  ;[0.15 0.15 0.15 0.5] Make the "E-icon" bob up and down over time...
  (Transformation|SetRelativeLocation (Variables|Default|GetIconE_p1) (Math|Vector|MakeVector _x _y (+ _z (* (Math|Trig|Sin(Radians) (* (Utilities|Time|GetGameTimeinSeconds) 1.0)) 5e+01))) false false)
  ;[0.15 0.15 0.15 0.5] If the switch is ON: make it look ON, else: make it look OFF...
  (if (Variables|Default|Getlever_on)
    (Rendering|Material|SetMaterial _switch 0 "/Game/MyContent/MyMaterials/M_LeverDown.M_LeverDown")
    (else
      (Rendering|Material|SetMaterial _switch 0 "/Game/MyContent/MyMaterials/M_LeverUp.M_LeverUp")))
  ;[0.15 0.15 0.15 0.5] If "E" (the player's interact button) is pressed and the player is within interacting/touching range: set [lever_on] and [lever_pressed] to TRUE.
  (if (and (and (Variables|Default|Gettouching_player) (Variables|/Game/ThirdPerson/Blueprints/BP_ThirdPersonCharacter.BP_ThirdPersonCharacter_C|Getplayer_interact (Variables|Default|Getlever_player_controller))) (not (Variables|Default|Getlever_on)))
    (Variables|/Game/ThirdPerson/Blueprints/BP_ThirdPersonCharacter.BP_ThirdPersonCharacter_C|Setplayer_interact (Variables|Default|Getlever_player_controller) false)
    (Variables|Default|Setlever_on true)
    (Variables|Default|Setlever_pressed true)))

(event EventBeginPlay
  ;[0.15 0.15 0.15 0.5] Enable inputs (so we can detect keypresses)...
  (Class|Actor|CreateInputComponent "/Script/Engine.InputComponent")
  (Input|EnableInput (Game|GetPlayerController 0))
  ;[0.15 0.15 0.15 0.5] Set state of all variables: [touching_player] are FALSE and [e_icon_centre] (the centre point from which the "E-icon" bobs up & down from) is at the present E-icon's position...
  (Variables|Default|Settouching_player false)
  (Variables|Default|Sete_icon_center (.Location (Math|Transform|BreakTransform (Transformation|GetRelativeTransform (Variables|Default|GetIconE_p1)))))
  ;[0.15 0.15 0.15 0.5] Hide the "E icon"
  (Rendering|ToggleVisibility (Variables|Default|GetIconE_p1) false))

(event Input|KeyboardEvents|E
  (params (Key :type Key%20Structure :default "None")))

(fn ConstructionScript)