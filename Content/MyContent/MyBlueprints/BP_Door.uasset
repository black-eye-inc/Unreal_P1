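; Interactable door that opens when the player presses interact inside its hitbox and closes itself after they leave.
; Overlap events track the player and toggle two E-key prompt icons.
; Tick polls the interact input and state flags, including DoorOpened as an opening trigger, to run separate open and reversed close timelines.
; MoveDoorTo fakes an edge hinge by rotating the mesh and offsetting its location with sine and cosine.
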(event OnComponentBeginOverlap(hitbox)
  (params (OverlappedComponent :type Primitive%20Component%20Object%20Reference) (OtherActor :type Actor%20Object%20Reference) (OtherComp :type Primitive%20Component%20Object%20Reference) (OtherBodyIndex :type Integer) (bFromSweep :type Boolean) (SweepResult :type Hit%20Result%20Structure%20%28by%20ref%29))
  ;[0.15 0.15 0.15 0.5] Upon a player entering touching range: if the door is [interactable], and not [open] or [opening]: make [door_touching_player] TRUE and make the "E-icon" visible.
  (Utilities|Casting|CastToBP_ThirdPersonCharacter OtherActor)
  (if (and (Variables|Default|Getdoor_interactable) (Math|Boolean|NORBoolean (Variables|Default|Getdoor_open) (Variables|Default|Getdoor_opening)))
    (Variables|Default|Setdoor_touching_player true)
    (Rendering|SetVisibility (Variables|Default|GeticonE_2) true false)))

(event OnComponentEndOverlap(hitbox)
  (params (OverlappedComponent :type Primitive%20Component%20Object%20Reference) (OtherActor :type Actor%20Object%20Reference) (OtherComp :type Primitive%20Component%20Object%20Reference) (OtherBodyIndex :type Integer))
  ;[0.15 0.15 0.15 0.5] Upon the player leaving: ensure [door_touching_player] is FALSE and the "E-icon" is invisible.
  (Utilities|Casting|CastToBP_ThirdPersonCharacter OtherActor)
  (Variables|Default|Setdoor_touching_player false)
  (Rendering|SetVisibility (Variables|Default|GeticonE_2) false false))

(event EventBeginPlay
  (bind _door (Variables|Default|Getdoor))
  (bind _returnvalue (Transformation|GetRelativeTransform _door))
  (bind (_location _rotation _scale) (Math|Transform|BreakTransform _returnvalue))
  (bind (_x _y) (Math|Vector|BreakVector _scale))
  ;[0.15 0.15 0.15 0.5] Declare [door_fill] (as FALSE) and work out constants [door_centre] and [door_hinge_distance]...
  (Variables|Default|Setdoor_closed false)
  (Variables|Default|Setdoor_open false)
  (Variables|Default|Setdoor_center _location)
  (Variables|Default|Setdoor_hinge_distance (* (/ (- _x _y) 2.0) 1e+02))
  ;[0.15 0.15 0.15 0.5] Hide our "E-icon"
  (Rendering|ToggleVisibility (Variables|Default|GeticonE_1) false))

(event EventTick
  (params (DeltaSeconds :type Float%20%28single-precision%29))
  ;[0.15 0.15 0.15 0.5] Every frame: if has been opened (by player or level manager, etc): run the door opening timeline, then set [door_open] to TRUE...
  (if (Variables|Default|Getdoor_opened)
    (Variables|Default|Setdoor_opened false)
    (bind _door_open_timeline (Timeline|Timeline_1 PlayFromStart)
      (:Update
        (CallFunction|MoveDoorto _door_open_timeline))
      (:Finished
        (Variables|Default|Setdoor_open true)
        (Variables|Default|Setdoor_opening false)))
    (else
      ;[0.15 0.15 0.15 0.5] upon [door_touching_player], door not currently opening and  [player_interact] with door: set [door_opening] and [door_opened] to TRUE and hide "E-icon"...
      (if (and (and (Variables|Default|Getdoor_touching_player) (not (Variables|Default|Getdoor_opening))) (Variables|/Game/ThirdPerson/Blueprints/BP_ThirdPersonCharacter.BP_ThirdPersonCharacter_C|Getplayer_interact (Variables|Default|Getdoor_player_controller)))
        (Variables|Default|Setdoor_opened true)
        (Variables|Default|Setdoor_opening true)
        (Rendering|SetVisibility (Variables|Default|GeticonE_2) false false)
        (else
          ;[0.15 0.15 0.15 0.5] If the door is open and is interactable, but the player isn't touching it and the door isn't currently being closed: set [door_closed] to TRUE and close the door.
          (if (and (and (Variables|Default|Getdoor_open) (Variables|Default|Getdoor_interactable)) (Math|Boolean|NORBoolean (Variables|Default|Getdoor_touching_player) (Variables|Default|Getdoor_closed)))
            (Variables|Default|Setdoor_closed true)
            (bind _door_open_timeline_2 (Timeline|Timeline_0 ReverseFromEnd)
              (:Update
                (CallFunction|MoveDoorto _door_open_timeline_2))
              (:Finished
                (Variables|Default|Setdoor_open false)
                (Variables|Default|Setdoor_closed false)))))))))

(fn ConstructionScript)

(fn MoveDoorto
  (params (angle%20%28radians%29 :type Float%20%28double-precision%29))
  (bind _door_center (Variables|Default|Getdoor_center))
  (bind _door_hinge_distance (Variables|Default|Getdoor_hinge_distance))
  (bind (_x _y _z) (Math|Vector|BreakVector _door_center))
  ;[0.15 0.15 0.15 0.5] rotate door...
  (Transformation|SetRelativeRotation (Variables|Default|Getdoor) (Math|Rotator|MakeRotator 0.0 0.0 angle%20%28radians%29) false false)
  ;[0.15 0.15 0.15 0.5] move door so that it looks like it's turning on a hinge
  (Transformation|SetRelativeLocation (Variables|Default|Getdoor) (Math|Vector|MakeVector (+ (- (Variables|Default|Getdoor_hinge_distance) (* (Math|Trig|Cos(Degrees) angle%20%28radians%29) _door_hinge_distance)) _x) (- _y (* _door_hinge_distance (Math|Trig|Sin(Degrees) angle%20%28radians%29))) _z) false false))